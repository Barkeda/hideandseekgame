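; BP_PlayerCharacter is the player character Blueprint that manages the health bar, exit menu and death screen.
; On BeginPlay it adds the health bar widget to the viewport.
; When HealthComp reports zero health, it waits briefly, shows the exit-game widget, pauses the game and switches to UI-only input with a cursor.
; The Menu input action opens the same widget with cursor and UI-only input, but does not pause.
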(event `self.ReceiveBeginPlay`
  (bind _returnvalue (`|CreateWidget` "/Game/_Game/HUD/Health_bar_UI.Health_bar_UI_C"))
  (`UserWidget.AddToViewport` _returnvalue 0))

(event `self.HealthComp.OnHealthChanged`
  (params (OwningHealthComp :type "HealthComponent Object Reference") (Health :type "Float (single-precision)") (HealthDelta :type "Float (single-precision)") (DamageType :type "DamageType Object Reference") (InstigatedBy :type "Controller Object Reference") (DamageCauser :type "Actor Object Reference"))
  (bind _returnvalue (`GameplayStatics.GetPlayerController` 0))
  (if (== Health 0.0)
    (`KismetSystemLibrary.Delay` 2.0)
    (bind _returnvalue_2 (`|CreateWidget` "/Game/_Game/HUD/ExitGame/ExitGame_UI.ExitGame_UI_C"))
    (`UserWidget.AddToViewport` _returnvalue_2 0)
    (`GameplayStatics.SetGamePaused` true)
    (`WidgetBlueprintLibrary.SetInputMode_UIOnlyEx` _returnvalue null)
    (set `PlayerController.bShowMouseCursor` true _returnvalue)))

(event `InputAction|Menu`
  (params (Key :type "Key Structure"))
  (bind _returnvalue (`GameplayStatics.GetPlayerController` 0))
  (:`Pressed`
    (bind _returnvalue_2 (`|CreateWidget` "/Game/_Game/HUD/ExitGame/ExitGame_UI.ExitGame_UI_C"))
    (`UserWidget.AddToViewport` _returnvalue_2 0)
    (`WidgetBlueprintLibrary.SetInputMode_UIOnlyEx` _returnvalue null)
    (set `PlayerController.bShowMouseCursor` true _returnvalue)))

(fn `UserConstructionScript`)