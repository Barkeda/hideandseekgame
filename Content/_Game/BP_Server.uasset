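; BP_Server is an interactable server actor that takes a key from the player when they interact while nearby.
; Overlapping its ServerBox enables the actor's input for player controller 0, and leaving disables it.
; Pressing Interact decrements NumberOfKeys on BP_PlayerCharacter if above zero and prints a key-lost message, with no other effect yet.
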(event `InputAction|Interact`
  (params (Key :type "Key Structure"))
  (:`Pressed`
    (bind _asbp_player_character (cast `/Game/_Game/PlayerCharacter/BP_PlayerCharacter` (`GameplayStatics.GetPlayerCharacter` 0)))
    (bind _numberofkeys (`/Game/_Game/PlayerCharacter/BP_PlayerCharacter.NumberOfKeys` _asbp_player_character))
    (if (> _numberofkeys 0)
      (`/Engine/EditorBlueprintResources/StandardMacros.DecrementInt` _numberofkeys
        (:`  `
          (`KismetSystemLibrary.PrintString` "Key lost"))))))

(event `self.ServerBox.OnComponentBeginOverlap`
  (params (OverlappedComponent :type "PrimitiveComponent Object Reference") (OtherActor :type "Actor Object Reference") (OtherComp :type "PrimitiveComponent Object Reference") (OtherBodyIndex :type Integer) (bFromSweep :type Boolean) (SweepResult :type "HitResult Structure (by ref)"))
  (if (== OtherActor (`GameplayStatics.GetPlayerCharacter` 0))
    (`self.EnableInput` (`GameplayStatics.GetPlayerController` 0))))

(event `self.ServerBox.OnComponentEndOverlap`
  (params (OverlappedComponent :type "PrimitiveComponent Object Reference") (OtherActor :type "Actor Object Reference") (OtherComp :type "PrimitiveComponent Object Reference") (OtherBodyIndex :type Integer))
  (if (== OtherActor (`GameplayStatics.GetPlayerCharacter` 0))
    (`self.DisableInput` (`GameplayStatics.GetPlayerController` 0))))

(fn `UserConstructionScript`)