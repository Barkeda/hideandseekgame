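; Keycard pickup for a server mission objective that adds to the player's key count and updates their current objective.
; Overlapping the trigger enables actor input and shows an interact widget; leaving it reverses both.
; Pressing Interact removes the keycard and mission marker, updates BP_PlayerCharacter, plays a sound and destroys the actor.
; An unconnected branch that would unhide an owning BP_Server never runs.
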(event `self.KeycardTrigger.OnComponentBeginOverlap`
  (params (OverlappedComponent :type "PrimitiveComponent Object Reference") (OtherActor :type "Actor Object Reference") (OtherComp :type "PrimitiveComponent Object Reference") (OtherBodyIndex :type Integer) (bFromSweep :type Boolean) (SweepResult :type "HitResult Structure (by ref)"))
  (if (== OtherActor (`GameplayStatics.GetPlayerCharacter` 0))
    (`self.EnableInput` (`GameplayStatics.GetPlayerController` 0))
    (bind _returnvalue (`|CreateWidget` "/Game/_Game/HUD/Interact_UI.Interact_UI_C"))
    (bind _output_get (set `self.InteractUI` _returnvalue))
    (`UserWidget.AddToViewport` _output_get 0)))

(event `InputAction|Interact`
  (params (Key :type "Key Structure"))
  (:`Pressed`
    (`/Engine/EditorBlueprintResources/StandardMacros.IsValid` (`self.Keycard`)
      (:`Is Valid`
        (`ActorComponent.K2_DestroyComponent` (`self.Keycard`))
        (bind _asbp_player_character (cast `/Game/_Game/PlayerCharacter/BP_PlayerCharacter` (`GameplayStatics.GetPlayerCharacter` 0)))
        (`/Engine/EditorBlueprintResources/StandardMacros.IncrementInt` (`/Game/_Game/PlayerCharacter/BP_PlayerCharacter.NumberOfKeys` _asbp_player_character)
          (:`  `
            (`ActorComponent.K2_DestroyComponent` (`self.MissionMarker`))
            (set `/Game/_Game/PlayerCharacter/BP_PlayerCharacter.CurrentObjective` (`self.Current Objective`) _asbp_player_character)
            (`GameplayStatics.PlaySound2D` "/Game/_Game/MissionObjective/sounds/Objective_Sound.Objective_Sound" 1.0 1.0 0.0 null null)
            (`self.K2_DestroyActor`)))))))

(event `self.KeycardTrigger.OnComponentEndOverlap`
  (params (OverlappedComponent :type "PrimitiveComponent Object Reference") (OtherActor :type "Actor Object Reference") (OtherComp :type "PrimitiveComponent Object Reference") (OtherBodyIndex :type Integer))
  (if (== OtherActor (`GameplayStatics.GetPlayerCharacter` 0))
    (`self.DisableInput` (`GameplayStatics.GetPlayerController` 0))
    (`Widget.RemoveFromParent` (`self.InteractUI`))))

(fn `UserConstructionScript`)